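; BP_Catapult is a catapult actor that fires through a Shoot event driven by a physics constraint.
; Shoot prints a debug message, then a DoOnce gate sets the constraint's angular orientation target to the firing pose and, after a delay, back to ready.
; After a second delay, SpawnCannonball adds a child actor component at the CannonnallPos relative transform, and the gate resets for the next shot.
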(event Custom|Shoot
  ;[1 1 1] Реализуйте механику выстрела
  (Development|PrintString "Catapult shot!")
  (Utilities|FlowControl|DoOnce false :!label _label
    (:Completed
      (Class|PhysicsConstraintComponent|SetAngularOrientationTarget (Variables|Default|GetPhysicsConstraint) (Variables|Default|GetIn%20Pos%20Target))
      (Utilities|FlowControl|Delay 1.0)
      (Class|PhysicsConstraintComponent|SetAngularOrientationTarget (Variables|Default|GetPhysicsConstraint) (Variables|Default|GetIn%20Pos%20Ready))
      (Utilities|FlowControl|Delay 1.0)
      (CallFunction|SpawnCannonball)
      (goto _label Reset))))

(fn ConstructionScript)

(fn SpawnCannonball
  (AddComponent|AddChildActorComponent false (Transformation|GetRelativeTransform (Variables|Default|GetCannonnallPos))))